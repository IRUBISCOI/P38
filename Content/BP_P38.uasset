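; BP_P38 is an actor, apparently a P-38 aircraft, that flies in a straight line while spinning its Left and Right components, likely the propellers.
; Each Tick rolls both components locally by RotateSpeed and offsets Body along world X by BodySpeed.
; Both motions scale by world delta seconds for frame-rate independence, and the movement does not sweep for collision or follow the actor's facing.
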(event `self.ReceiveTick`
  (params (DeltaSeconds :type "Float (single-precision)"))
  (`SceneComponent.K2_AddLocalRotation` (`self.Left`) (`KismetMathLibrary.MakeRotator` (* (`self.RotateSpeed`) (`GameplayStatics.GetWorldDeltaSeconds`))) false false)
  (`SceneComponent.K2_AddLocalRotation` (`self.Right`) (`KismetMathLibrary.MakeRotator` (* (`self.RotateSpeed`) (`GameplayStatics.GetWorldDeltaSeconds`))) false false)
  (`SceneComponent.K2_AddWorldOffset` (`self.Body`) (`KismetMathLibrary.MakeVector` (* (`self.BodySpeed`) (`GameplayStatics.GetWorldDeltaSeconds`))) false false))

(fn `UserConstructionScript`)