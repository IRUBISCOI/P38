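; Player-controlled P-38 plane pawn that pitches, rolls, boosts and fires rockets.
; Pitch and Roll axes rotate the actor locally, scaled by frame time, while Boost switches FloatingPawnMovement's max speed between boost and normal values.
; Tick spins the Left and Right components around their roll axis and adds forward movement input, though its scale is zero.
; Shoot spawns BP_Rocket at the actor's location and rotation.
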(event `InputAxis|Pitch`
  (params (AxisValue :type "Float (single-precision)"))
  (`self.K2_AddActorLocalRotation` (`KismetMathLibrary.MakeRotator` 0.0 (* (`KismetMathLibrary.FClamp` AxisValue -1.0 1.0) (`GameplayStatics.GetWorldDeltaSeconds`) (`self.RotationSpeed`)))))

(event `InputAction|Boost`
  (params (Key :type "Key Structure"))
  (:`Pressed`
    (set `FloatingPawnMovement.MaxSpeed` (`self.BoostSpeed`) (`self.FloatingPawnMovement`)))
  (:`Released`
    (set `FloatingPawnMovement.MaxSpeed` (`self.MoveSpeed`) (`self.FloatingPawnMovement`))))

(event `InputAxis|Roll`
  (params (AxisValue :type "Float (single-precision)"))
  (`self.K2_AddActorLocalRotation` (`KismetMathLibrary.MakeRotator` (* (`KismetMathLibrary.FClamp` AxisValue -1.0) (`GameplayStatics.GetWorldDeltaSeconds`) (`self.RotationSpeed`)))))

(event `InputAction|Shoot`
  (params (Key :type "Key Structure"))
  (bind (_returnvalue_location _returnvalue_rotation) (`KismetMathLibrary.BreakTransform` (`self.GetTransform`)))
  (:`Pressed`
    (`|SpawnActorFromClass` "/Game/Blueprints/BP_Rocket.BP_Rocket_C" (`KismetMathLibrary.MakeTransform` _returnvalue_location _returnvalue_rotation) "Undefined" "OverrideRootScale" null null)))

(event `self.ReceiveBeginPlay`
  (`self.EnableInput` (`GameplayStatics.GetPlayerController` 0)))

(event `self.ReceiveTick`
  (params (DeltaSeconds :type "Float (single-precision)"))
  ;[1 1 1] Left Rotate
  (`SceneComponent.K2_AddLocalRotation` (`self.Left`) (`KismetMathLibrary.MakeRotator` (* (`self.RotateSpeed`) (`GameplayStatics.GetWorldDeltaSeconds`))) false false)
  ;[1 1 1] Right Rotate
  (`SceneComponent.K2_AddLocalRotation` (`self.Right`) (`KismetMathLibrary.MakeRotator` (* (`self.RotateSpeed`) (`GameplayStatics.GetWorldDeltaSeconds`))) false false)
  (`self.AddMovementInput` (`self.GetActorForwardVector`) 0.0))

(fn `UserConstructionScript`)